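; Mod actor for AdvancedFilter that patches the main menu's multiplayer UI, adding a Search widget and exposing server creation with a 32-player maximum.
; Every Tick it finds all W_MainMenu widgets and reapplies the changes, swapping the first row's contents for Search only when absent.
; Custom events can start or stop a looping timer running the same patch, but nothing here calls them.
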(event `暂停设置`
  (`KismetSystemLibrary.K2_ClearAndInvalidateTimerHandle` (stale `开始设置` _returnvalue)))

(event `开始设置`
  (bind _returnvalue (`KismetSystemLibrary.K2_SetTimerDelegate` (delegate `设置MainMenu`) 3.0 true)))

(event `设置MainMenu`
  (bind _foundwidgets (`WidgetBlueprintLibrary.GetAllWidgetsOfClass` "/Game/MainMenu/Widgets/MainMenu/W_MainMenu.W_MainMenu_C" false))
  (for _array_element _foundwidgets
    (`|ExecutionSequence`
      (:`then_0`
        (`Widget.SetVisibility` (`/Game/MainMenu/Widgets/MainMenu/W_MainMenu.VerticalBox_NavMultiplayer` _array_element) "Visible")
        (`Widget.SetVisibility` (`/Game/MainMenu/Widgets/MainMenu/W_MainMenu.Button_CreateServer` _array_element) "Visible")
        (`Widget.SetIsEnabled` (`/Game/MainMenu/Widgets/MainMenu/W_MainMenu.Button_CreateServer` _array_element) true))
      (:`then_1`
        (bind _w_createserver (`/Game/MainMenu/Widgets/MainMenu/W_MainMenu.W_CreateServer` _array_element))
        (set `/Game/MainMenu/Widgets/MainMenu/W_CreateServer.MaximumPlayers` 32 _w_createserver)
        (`TextBlock.SetText` (`/Game/MainMenu/Widgets/MainMenu/W_CreateServer.TextBlock_Error` _w_createserver) "Max Player 32"))
      (:`then_2`
        (bind _verticalbox_multiplayer (`/Game/MainMenu/Widgets/MainMenu/W_MainMenu.VerticalBox_Multiplayer` _array_element))
        (bind _returnvalue (`PanelWidget.GetChildAt` _verticalbox_multiplayer 0))
        (bind `_as水平框` (cast `HorizontalBox` _returnvalue))
        (cast `/Game/Mods/AdvancedFilter_P/Search` (`PanelWidget.GetChildAt` `_as水平框` 0)
          (:`then`
            (`Widget.RemoveFromParent` (`|GetArrayItem` (`PanelWidget.GetAllChildren` `_as水平框`) 1)))
          (:`CastFailed`
            (`Widget.SetVisibility` (`PanelWidget.GetChildAt` _verticalbox_multiplayer 2) "Collapsed")
            (`Widget.RemoveFromParent` (`PanelWidget.GetAllChildren` `_as水平框`))
            (bind _returnvalue_2 (`|CreateWidget` "/Game/Mods/AdvancedFilter_P/Search.Search_C" null _array_element))
            (`PanelWidget.AddChild` `_as水平框` _returnvalue_2)
            (`Widget.SetVisibility` _returnvalue "Visible")
            (bind _returnvalue_3 (`WidgetLayoutLibrary.SlotAsHorizontalBoxSlot` _returnvalue_2))
            (`HorizontalBoxSlot.SetHorizontalAlignment` _returnvalue_3 "HAlign_Fill")
            (`HorizontalBoxSlot.SetVerticalAlignment` _returnvalue_3 "VAlign_Top")
            (`HorizontalBoxSlot.SetSize` _returnvalue_3 (make `SlateChildSize` 1.0))))))))

(event `self.ReceiveBeginPlay`)

(event `self.ReceiveTick`
  (params (DeltaSeconds :type "Float (single-precision)"))
  (`self.设置MainMenu`))

(event `self.ReceiveDestroyed`)

(fn `UserConstructionScript`
  (`parent.UserConstructionScript`))